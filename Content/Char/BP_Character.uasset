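; Player character with axis-driven movement and look, a toggleable spotlight on F, and an E trace that sends a grab message through BPI_Take.
; A received Celsia temperature is stored and forwarded as text to the TAB actor.
; Delayed Tick branches turn that temperature into a frost density on a dynamic post-process material on the camera, and drive a timeline that widens FOV while moving.
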(event Custom|ChanFOV
  ;[1 0.5387 0 0.3 48] MoveMent
  ;;[0 0.4754 1 0.7 16] Walk
  (if (!= (Math|Vector|VectorLength (Transformation|GetVelocity)) 0.0)
    (bind _alpha (Timeline|ChangerFOV Play)
      (:Update
        (Camera|SetFieldOfView (Variables|Default|GetCamera) (Math|Float|Lerp 75.0 8e+01 _alpha))))
    (else
      (Timeline|ChangerFOV Reverse))))

(event Custom|FEffect
  (Rendering|Material|SetScalarParameterValue (Variables|Default|GetDynamicPostProcess) "Density" (Variables|Default|GetFrozen_Effect) :!class /Script/Engine.MaterialInstanceDynamic))

(event EventTick
  (params (DeltaSeconds :type Float%20%28single-precision%29))
  (Utilities|FlowControl|Sequence
    (:then_0
      (Utilities|FlowControl|Delay 0.2)
      (|SetFreeze))
    (:then_1
      (Utilities|FlowControl|Delay 0.2)
      (CallFunction|ChanFOV)
      (Rendering|Material|SetScalarParameterValue (Variables|Default|GetDynamicPostProcess) "Density" (Variables|Default|GetFrozen_Effect) :!class /Script/Engine.MaterialInstanceDynamic))))

(event EventFloatSettings
  (params (Celsia :type Float%20%28double-precision%29))
  (Utilities|FlowControl|Delay 0.2)
  (Utilities|FlowControl|Sequence
    (:then_0
      (Variables|Default|SetCelsia Celsia))
    (:then_1
      (bind _returnvalue (Actor|GetActorOfClass "/Game/Char/TAB.TAB_C"))
      (Class|BPIWarm|TABc(Message) _returnvalue (Utilities|Text|ToText(Float) (Variables|Default|GetCelsia) "HalfToEven")))))

(event EventBeginPlay
  (bind _returnvalue (Rendering|Material|CreateDynamicMaterialInstance "/Game/Char/Widgets/CameraEffects/Frozenmat/Mat_FrozenEffect.Mat_FrozenEffect" "None" "None" :!class /Script/Engine.KismetMaterialLibrary))
  (bind _output_get (Variables|Default|SetDynamicPostProcess _returnvalue))
  (Utilities|Struct|SetmembersinPostProcessSettings (Variables|/Script/Engine.CameraComponent|GetPostProcessSettings (Variables|Default|GetCamera)) (Utilities|Struct|MakeWeightedBlendables (Utilities|Array|MakeArray (Utilities|Struct|MakeWeightedBlendable 1.0 _output_get))))
  (CallFunction|FEffect))

(event EventInventoryAdd
  (params (Item :type Actor%20Object%20Reference)))

(event Input|AxisEvents|InputAxisRight_Cont
  (params (AxisValue :type Float%20%28single-precision%29))
  ;[1 0.5387 0 0.3 48] MoveMent
  ;;[1 0 0.1047 1 24] BasicMovement
  ;;;[1 0 0.434 0.2 16] WASD
  (Pawn|Input|AddMovementInput (Transformation|GetActorRightVector) AxisValue false))

(event Input|AxisEvents|InputAxisFront_Cont
  (params (AxisValue :type Float%20%28single-precision%29))
  ;[1 0.5387 0 0.3 48] MoveMent
  ;;[1 0 0.1047 1 24] BasicMovement
  ;;;[1 0 0.434 0.2 16] WASD
  (Pawn|Input|AddMovementInput (Transformation|GetActorForwardVector) AxisValue false))

(event Input|AxisEvents|InputAxisMouseCont_RL
  (params (AxisValue :type Float%20%28single-precision%29))
  ;[1 0.5387 0 0.3 48] MoveMent
  ;;[1 0 0.1047 1 24] BasicMovement
  ;;;[1 0.4024 0 0.2 16] CameraMove
  (Pawn|Input|AddControllerYawInput AxisValue))

(event Input|AxisEvents|InputAxisMouseCont_UD
  (params (AxisValue :type Float%20%28single-precision%29))
  ;[1 0.5387 0 0.3 48] MoveMent
  ;;[1 0 0.1047 1 24] BasicMovement
  ;;;[1 0.4024 0 0.2 16] CameraMove
  (Pawn|Input|AddControllerPitchInput AxisValue))

(event Input|KeyboardEvents|E
  (params (Key :type Key%20Structure :default "None"))
  (bind (_startvec _endvec) (|GetVectors))
  ;[1 0.3112 0.3511] Take
  (:Released
    (bind (_outhit _returnvalue) (Collision|LineTraceByChannel _startvec _endvec "TraceTypeQuery1" false 0 "ForDuration"))
    (if _returnvalue
      (bind _outactors (Actor|GetAllActorswithInterface "/Game/Char/BPIs/BPI_Take.BPI_Take_C"))
      (bind _array_element (Utilities|Array|ForEachLoopwithBreak _outactors :!label _label)
        (:LoopBody
          (if (== _array_element (.HitActor (Collision|BreakHitResult _outhit)))
            (goto _label Break)))
        (:Completed
          (Class|BPITake|Grab(Message) _array_element))))))

(event Input|KeyboardEvents|F
  (params (Key :type Key%20Structure :default "None"))
  ;[1 1 1] LightSpot
  (:Released
    (Utilities|FlowControl|FlipFlop
      (:A
        (bind _alpha (Timeline|LightSpot Play)
          (:Update
            (Rendering|Components|Light|SetIntensity (Variables|Default|GetSpotLight) (Math|Float|Lerp 2e+04 0.0 _alpha)))))
      (:B
        (Timeline|LightSpot ReverseFromEnd)))))

(fn ConstructionScript)